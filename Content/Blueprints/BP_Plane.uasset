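; Player plane attached to BP_FoxVRPawn that follows a VR motion-controller hand and fires projectiles on a looping timer.
; Switching hands dashes it across with eased interpolation, damaging overlapped actors until the dash nears completion, when hand rotation and laser pointer return.
; Tick also drives curve-based barrel rolls and speed-scaled thruster particles.
; Damage or world-static hits shake the ship and reduce PlayerState health, destroying it at zero.
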(event OnComponentBeginOverlap(ShipBodyMesh)
  (params (OverlappedComponent :type Primitive%20Component%20Object%20Reference) (OtherActor :type Actor%20Object%20Reference) (OtherComp :type Primitive%20Component%20Object%20Reference) (OtherBodyIndex :type Integer) (bFromSweep :type Boolean) (SweepResult :type Hit%20Result%20Structure%20%28by%20ref%29))
  ;[1 1 1] Overlap handler
  (Utilities|IsValid OtherComp
    (:Is%20Valid
      (if (Utilities|Enum|Equal(Enum) (Collision|GetCollisionObjectType OtherComp) "ECC_WorldStatic")
        (CallFunction|TakeDamage 1)))))

(event Custom|TakeDamage
  (params (Damage :type Integer))
  ;[1 1 1] Damage handler
  (if (not (Audio|Components|Audio|IsPlaying (Variables|Default|GetDamageShakeTimeline)))
    (Utilities|FlowControl|Sequence
      (:then_0
        (bind _rotation (Timeline|DamageShakeTimeline PlayFromStart)
          (:Update
            (Transformation|SetRelativeRotation (Variables|Default|GetDamageShakeWrapper) (Math|Rotator|MakeRotator (.x _rotation) (.y _rotation) (.z _rotation)) false false))))
      (:then_1
        (bind _asbp_fox_vrpawn (Utilities|Casting|CastToBP_FoxVRPawn (Actor|GetAttachParentActor)))
        (bind _asbp_fox_vrplayer_state (Utilities|Casting|CastToBP_FoxVRPlayerState (Variables|/Script/Engine.Pawn|GetPlayerState _asbp_fox_vrpawn)))
        (bind _output_get (Variables|/Game/Blueprints/GameplayFramework/BP_FoxVRPlayerState.BP_FoxVRPlayerState_C|SetHealth _asbp_fox_vrplayer_state (- (Variables|/Game/Blueprints/GameplayFramework/BP_FoxVRPlayerState.BP_FoxVRPlayerState_C|GetHealth _asbp_fox_vrplayer_state) Damage)))
        (if (<= _output_get 0)
          (Actor|DestroyActor))))))

(event Custom|StartFiring
  (bind _returnvalue (Utilities|Time|SetTimerbyEvent (delegate Custom|Refire) (Variables|Default|GetTimeBetweenShots) true))
  (Variables|Default|SetRefireTimerHandle _returnvalue))

(event Custom|StopFiring
  (Utilities|Time|ClearandInvalidateTimerbyHandle (Variables|Default|GetRefireTimerHandle)))

(event Custom|Refire
  (bind _gunbarrelscene (Variables|Default|GetGunBarrelScene))
  (bind _returnvalue (Transformation|GetWorldTransform _gunbarrelscene))
  (bind _returnvalue_2 (Game|SpawnActorfromClass (Variables|Default|GetProjectileClass) (Math|Transform|MakeTransform (.location _returnvalue) (.rotation _returnvalue) "1.000000,1,1") "AlwaysSpawn" 0 (Variables|Actor|GetInstigator)))
  (Transformation|AttachActorToActor _returnvalue_2 (Actor|GetAttachParentActor) "None" "KeepWorld" "KeepWorld" "KeepWorld" true))

(event EventTick
  (params (DeltaSeconds :type Float%20%28single-precision%29))
  (bind _thrustparticles (Variables|Default|GetThrustParticles))
  (bind _targethandcomponent (Variables|Default|GetTargetHandComponent))
  (Utilities|FlowControl|Sequence
    (:then_0
      (Utilities|FlowControl|Sequence
        (:then_0
          (Variables|Default|SetBarrelRollInterpAlpha (Math|Interpolation|FInterptoConstant (Variables|Default|GetBarrelRollInterpAlpha) (Variables|Default|GetBarrelRollTarget) (Utilities|Time|GetWorldDeltaSeconds) (Variables|Default|GetBarrelRollInterpSpeed))))
        (:then_1
          (Transformation|SetRelativeRotation (Variables|Default|GetBarrelRollWrapper) (Math|Rotator|MakeRotator (* (Math|Curves|GetFloatValue (Variables|Default|GetBarrelRollCurve) (Variables|Default|GetBarrelRollInterpAlpha)) (Variables|Default|GetBarrelRollSign)) 0.0 0.0) false false))
        (:then_2
          (bind _asbp_fox_vrpawn (Utilities|Casting|CastToBP_FoxVRPawn (Actor|GetAttachParentActor)))
          (Effects|Components|ParticleSystem|SetVectorParameter _thrustparticles "Intensity" (Math|Vector|MakeVector (Math|Float|MapRangeClamped (/ (Variables|/Game/Blueprints/BP_FoxVRPawn.BP_FoxVRPawn_C|GetSplineVelocity _asbp_fox_vrpawn) (Variables|/Game/Blueprints/BP_FoxVRPawn.BP_FoxVRPawn_C|GetMaxSplineVelocity _asbp_fox_vrpawn)) 0.0 1.0 0.0 -1e+03) 0.0 0.0))
          (Effects|Components|ParticleSystem|SetVectorParameter _thrustparticles "CoronaSize" (Math|Vector|MakeVector (Math|Float|MapRangeClamped (/ (Variables|/Game/Blueprints/BP_FoxVRPawn.BP_FoxVRPawn_C|GetSplineVelocity _asbp_fox_vrpawn) (Variables|/Game/Blueprints/BP_FoxVRPawn.BP_FoxVRPawn_C|GetMaxSplineVelocity _asbp_fox_vrpawn)) 0.0 1.0 2e+01 8e+01) (Math|Float|MapRangeClamped (/ (Variables|/Game/Blueprints/BP_FoxVRPawn.BP_FoxVRPawn_C|GetSplineVelocity _asbp_fox_vrpawn) (Variables|/Game/Blueprints/BP_FoxVRPawn.BP_FoxVRPawn_C|GetMaxSplineVelocity _asbp_fox_vrpawn)) 0.0 1.0 2e+01 8e+01) (Math|Float|MapRangeClamped (/ (Variables|/Game/Blueprints/BP_FoxVRPawn.BP_FoxVRPawn_C|GetSplineVelocity _asbp_fox_vrpawn) (Variables|/Game/Blueprints/BP_FoxVRPawn.BP_FoxVRPawn_C|GetMaxSplineVelocity _asbp_fox_vrpawn)) 0.0 1.0 2e+01 8e+01))))))
    (:then_1
      ;[1 1 1] Hand-specific behaviour
      (Utilities|IsValid (Variables|Default|GetActiveHandComponent)
        (:Is%20Valid
          (Utilities|FlowControl|Sequence
            (:then_0
              (Variables|Default|SetCachedDashInterpAlpha (Variables|Default|GetDashInterpAlpha))
              (bind _output_get (Variables|Default|SetDashInterpAlpha (Math|Interpolation|FInterpTo (Variables|Default|GetDashInterpAlpha) 1.0 (Utilities|Time|GetWorldDeltaSeconds) (Variables|Default|GetMoveInterpSpeed))))
              (if (and (>= _output_get 0.8) (< (Variables|Default|GetCachedDashInterpAlpha) 0.8))
                (CallFunction|ResetRotationInterpolation)
                (CallFunction|SetLaserPointerVisible true)
                (Variables|Default|SetUseHandRotation true)
                (Variables|Default|SetApplyDashDamage false)))
            (:then_1
              (Transformation|SetRelativeLocation (Variables|Default|GetRootScene) (Math|Vector|Lerp(Vector) (Variables|Default|GetDashStartPoint) (CallFunction|GetHandRelativeLocation (Variables|Default|GetActiveHandComponent)) (Variables|Default|GetDashInterpAlpha)) false false))
            (:then_2
              (if (Variables|Default|GetUseHandRotation)
                (Variables|Default|SetTargetEndRotation (Transformation|GetWorldRotation (Variables|Default|GetActiveHandComponent)))
                (else
                  (Utilities|IsValid _targethandcomponent
                    (:Is%20Valid
                      (Variables|Default|SetTargetEndRotation (Math|Rotator|FindLookatRotation (Variables|/Script/Engine.SceneComponent|GetRelativeLocation (Variables|Default|GetRootScene)) (CallFunction|GetHandRelativeLocation _targethandcomponent))))))))
            (:then_3
              (Variables|Default|SetTargetInterpAlpha (Math|Interpolation|FInterpTo (Variables|Default|GetTargetInterpAlpha) 1.0 (Utilities|Time|GetWorldDeltaSeconds) (Variables|Default|GetMoveInterpSpeed))))
            (:then_4
              (Transformation|SetActorRotation (Math|Rotator|Lerp(Rotator) (Variables|Default|GetTargetStartRotation) (Variables|Default|GetTargetEndRotation) (Variables|Default|GetTargetInterpAlpha) true)))))))))

(event Collision|EventActorBeginOverlap
  (params (OtherActor :type Actor%20Object%20Reference))
  (if (Variables|Default|GetApplyDashDamage)
    (Game|Damage|ApplyDamage OtherActor (Variables|Default|GetDashDamage) (Game|GetInstigatorController) self)))

(fn ConstructionScript)

(fn SwitchtoTargetHand
  (Variables|Default|SetActiveHandComponent (Variables|Default|GetTargetHandComponent))
  (Variables|Default|SetTargetHandComponent 0)
  (CallFunction|ResetLocationInterpolation)
  (Variables|Default|SetApplyDashDamage true))

(fn SetTargetHand
  (params (TargetHand :type Scene%20Component%20Object%20Reference))
  (Variables|Default|SetTargetHandComponent TargetHand)
  (CallFunction|ResetRotationInterpolation)
  (CallFunction|SetLaserPointerVisible false)
  (Variables|Default|SetUseHandRotation false))

(fn ResetRotationInterpolation
  (Variables|Default|SetTargetInterpAlpha 0.0)
  (Variables|Default|SetTargetStartRotation (Transformation|GetActorRotation)))

(fn SetActiveHand
  (params (ActiveHand :type Scene%20Component%20Object%20Reference))
  (Variables|Default|SetActiveHandComponent ActiveHand)
  (Variables|Default|SetTargetHandComponent 0)
  (CallFunction|ResetLocationInterpolation)
  (CallFunction|ResetRotationInterpolation)
  (CallFunction|SetLaserPointerVisible true))

(fn ResetLocationInterpolation
  (Variables|Default|SetDashInterpAlpha 0.0)
  (Variables|Default|SetDashStartPoint (Variables|/Script/Engine.SceneComponent|GetRelativeLocation (Variables|Default|GetRootScene))))

(fn BarrelRoll
  (params (Clockwise :type Boolean))
  (Variables|Default|SetBarrelRollInterpAlpha 0.0)
  (Variables|Default|SetBarrelRollTarget 1.0)
  (Variables|Default|SetBarrelRollSign (Math|Float|SelectFloat 1.0 -1.0 Clockwise)))

(fn SetLaserPointerVisible
  (params (Visible :type Boolean))
  (Development|SetHiddeninGame (Variables|Default|GetLaserPointer) (not Visible) false))

(fn IsInvincible
  (return (or (< (Variables|Default|GetBarrelRollInterpAlpha) (Variables|Default|GetBarrelRollInvincibilityThreshold)) (< (Variables|Default|GetDashInterpAlpha) (Variables|Default|GetDashInvincibilityThreshold)))))

(fn GetHandRelativeLocation
  (params (Hand :type Scene%20Component%20Object%20Reference))
  (return (- (Transformation|GetWorldLocation Hand) (Transformation|GetActorLocation (Actor|GetAttachParentActor)))))
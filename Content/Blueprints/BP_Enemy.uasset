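; BP_Enemy is a flying enemy for a Fox VR game that moves at a constant local velocity and attacks the player's plane.
; Tick sets IsFiring while the player pawn is within AggroRadius and facing the enemy's side.
; Its RepNotify toggles a looping timer for refiring projectiles aimed at the plane.
; Any damage destroys it and credits the instigator's HitCount, while overlapping a plane damages that plane.
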(event Custom|Refire
  (bind _returnvalue (Transformation|GetActorLocation))
  (bind _asbp_fox_vrpawn (Utilities|Casting|CastToBP_FoxVRPawn (Game|Player|GetPlayerPawn 0)))
  (Utilities|IsValid (Variables|/Game/Blueprints/BP_FoxVRPawn.BP_FoxVRPawn_C|GetPlaneActor _asbp_fox_vrpawn)
    (:Is%20Valid
      (Game|SpawnActorfromClass "/Game/Blueprints/BP_EnemyProjectile.BP_EnemyProjectile_C" (Math|Transform|MakeTransform _returnvalue (Math|Rotator|FindLookatRotation _returnvalue (Transformation|GetActorLocation (Variables|/Game/Blueprints/BP_FoxVRPawn.BP_FoxVRPawn_C|GetPlaneActor _asbp_fox_vrpawn))) "1,1,1") "Undefined" 0 0))))

(event Game|Damage|EventAnyDamage
  (params (Damage :type Float%20%28single-precision%29) (DamageType :type Damage%20Type%20Object%20Reference) (InstigatedBy :type Controller%20Object%20Reference) (DamageCauser :type Actor%20Object%20Reference))
  (Utilities|FlowControl|Sequence
    (:then_0
      (bind _asbp_fox_vrplayer_state (Utilities|Casting|CastToBP_FoxVRPlayerState (Variables|/Script/Engine.Controller|GetPlayerState InstigatedBy)))
      (Math|Integer|IncrementInt (Variables|/Game/Blueprints/GameplayFramework/BP_FoxVRPlayerState.BP_FoxVRPlayerState_C|GetHitCount _asbp_fox_vrplayer_state)))
    (:then_1
      (Actor|DestroyActor))))

(event Collision|EventActorBeginOverlap
  (params (OtherActor :type Actor%20Object%20Reference))
  (bind _asbp_plane (Utilities|Casting|CastToBP_Plane OtherActor))
  (Default|TakeDamage _asbp_plane 1))

(event EventTick
  (params (DeltaSeconds :type Float%20%28single-precision%29))
  (bind _returnvalue (Game|Player|GetPlayerPawn 0))
  (bind _returnvalue_2 (Transformation|GetActorLocation))
  (bind _returnvalue_3 (Transformation|GetActorLocation _returnvalue))
  (bind _returnvalue_4 (- _returnvalue_3 _returnvalue_2))
  (Transformation|AddActorWorldOffset (* (Math|Vector|RotateVector (Variables|Default|GetVelocity) (Transformation|GetActorRotation)) DeltaSeconds))
  (Utilities|IsValid _returnvalue
    (:Is%20Valid
      (if (and (<= (Math|Vector|DotProduct _returnvalue_4 (Transformation|GetActorForwardVector _returnvalue)) 0.0) (<= (Math|Vector|VectorLength _returnvalue_4) (Variables|Default|GetAggroRadius)))
        (if (not (Variables|Default|GetIsFiring))
          (Variables|Default|SetIsFiring true))
        (elif (Variables|Default|GetIsFiring)
          (Variables|Default|SetIsFiring false))))))

(fn ConstructionScript)

(fn OnRepIsFiring
  (if (Variables|Default|GetIsFiring)
    (bind _returnvalue (Utilities|Time|SetTimerbyEvent (EventDispatchers|CreateEvent :!event Custom|Refire) (Variables|Default|GetRefireDuration) true))
    (Variables|Default|SetRefireTimerHandle _returnvalue)
    (else
      (Utilities|Time|ClearandInvalidateTimerbyHandle (Variables|Default|GetRefireTimerHandle)))))
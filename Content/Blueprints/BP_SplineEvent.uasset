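; Spline event actor that places a trigger on the motion spline, with an empty Trigger event as a stub for the response.
; The construction script looks up the motion spline, stores it, then moves SpawnTrigger to the spline point closest to the actor and detaches it, keeping its world transform.
; A beam particle, LineVisualization, links the actor to SpawnTrigger to show the connection.
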(event Custom|Trigger)

(fn ConstructionScript
  (bind _spawntrigger (Variables|Default|GetSpawnTrigger))
  (bind _linevisualization (Variables|Default|GetLineVisualization))
  (bind _spline (Utilities|GetMotionSpline)
    (:Success
      (Variables|Default|SetSplinePath _spline)
      (Utilities|FlowControl|Sequence
        (:then_0
          (Transformation|SetWorldLocation _spawntrigger (Spline|FindLocationClosesttoWorldLocation (Variables|/Game/Blueprints/BP_SplineActor.BP_SplineActor_C|GetSpline (Variables|Default|GetSplinePath)) (Transformation|GetActorLocation) "World") false false)
          (Transformation|DetachFromComponent _spawntrigger "KeepWorld" "KeepWorld" "KeepWorld" true))
        (:then_1
          (Class|ParticleSystemComponent|SetBeamSourcePoint _linevisualization 0 (Transformation|GetActorLocation))
          (Class|ParticleSystemComponent|SetBeamTargetPoint _linevisualization 0 (Transformation|GetWorldLocation (Variables|Default|GetSpawnTrigger))))))))
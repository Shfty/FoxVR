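; BP_EnemySpawnLine is an enemy spawn point variant that lays out spawn transforms in a straight, evenly spaced line.
; Its construction script rebuilds SpawnTransforms from Count and Distance along the selected X, Y or Z axis, starting at zero offset with no rotation and unit scale.
; Mirror adds a negated copy of every non-zero index, extending the line both ways.
; The parent construction script runs after the array is filled.
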(event EventBeginPlay)

(event Collision|EventActorBeginOverlap
  (params (OtherActor :type Actor%20Object%20Reference)))

(event EventTick
  (params (DeltaSeconds :type Float%20%28single-precision%29)))

(fn ConstructionScript
  (|SetBy-RefVar (Variables|Default|GetSpawnTransforms) (Utilities|Array|MakeArray))
  (for _index (range 0 (- (Variables|Default|GetCount) 1))
    (Utilities|Array|Add (Variables|Default|GetSpawnTransforms) (Math|Transform|MakeTransform (Utilities|Select :Index (Variables|Default|GetAxis) :X (Math|Vector|MakeVector (* (Math|Conversions|ToFloat(Integer) _index) (Variables|Default|GetDistance)) 0.0 0.0) :Y (Math|Vector|MakeVector 0.0 (* (Math|Conversions|ToFloat(Integer) _index) (Variables|Default|GetDistance)) 0.0) :Z (Math|Vector|MakeVector 0.0 0.0 (* (Math|Conversions|ToFloat(Integer) _index) (Variables|Default|GetDistance)))) "0, 0, 0" "1,1,1"))
    (if (and (!= _index 0) (Variables|Default|GetMirror))
      (Utilities|Array|Add (Variables|Default|GetSpawnTransforms) (Math|Transform|MakeTransform (* (Utilities|Select :Index (Variables|Default|GetAxis) :X (Math|Vector|MakeVector (* (Math|Conversions|ToFloat(Integer) _index) (Variables|Default|GetDistance)) 0.0 0.0) :Y (Math|Vector|MakeVector 0.0 (* (Math|Conversions|ToFloat(Integer) _index) (Variables|Default|GetDistance)) 0.0) :Z (Math|Vector|MakeVector 0.0 0.0 (* (Math|Conversions|ToFloat(Integer) _index) (Variables|Default|GetDistance)))) -1.0) "0, 0, 0" "1,1,1"))))
  (|CallParentFunction))
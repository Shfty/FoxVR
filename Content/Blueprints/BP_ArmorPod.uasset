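; BP_ArmorPod is a hand-attached pod with spinning spikes that switches between deflection and attack by how fast it moves.
; Tick infers velocity relative to the parent actor, toggling attack and deflection spheres and crossfading shield particles against a deflection billboard.
; Overlapping a BP_Enemy during attack applies damage.
; When replicated ActiveHandComponent changes to a valid component, timelines shrink the pod, reattach it there and scale it back in.
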(event Custom|Disappear
  (bind _value (Timeline|DisappearTimeline PlayFromStart)
    (:Update
      (Transformation|SetActorScale3D (Math|Conversions|ToVector(Float) _value)))
    (:Finished
      (Transformation|AttachComponentToComponent (Variables|Default|GetActiveHandComponent) "None" "SnapToTarget" "SnapToTarget" "SnapToTarget" true)
      (bind _value_2 (Timeline|AppearTimeline PlayFromStart)
        (:Update
          (Transformation|SetActorScale3D (Math|Conversions|ToVector(Float) _value_2)))))))

(event EventBeginPlay
  (Transformation|AttachComponentToComponent (Variables|Default|GetShieldParticles) (VehicleSound|GetRootComponent (Actor|GetAttachParentActor)) "None" "SnapToTarget" "SnapToTarget" "SnapToTarget" false)
  (bind _returnvalue (Rendering|Material|CreateDynamicMaterialInstance (Variables|Default|GetDeflectionBillboard) 0 "/Game/Materials/M_RadialGradientParticle.M_RadialGradientParticle" :!class /Script/Engine.PrimitiveComponent))
  (Variables|Default|SetRadialGradientMID _returnvalue))

(event EventTick
  (params (DeltaSeconds :type Float%20%28single-precision%29))
  (bind _shieldparticles (Variables|Default|GetShieldParticles))
  (Utilities|FlowControl|Sequence
    (:then_0
      ;[1 1 1] Rotate spikes
      (Transformation|AddRelativeRotation (Variables|Default|GetSpikeWrapper) (Math|Rotator|MakeRotator (* (Utilities|Time|GetWorldDeltaSeconds) 45.0) 0.0 0.0) false false))
    (:then_1
      ;[1 1 1] Calculate inferred velocity
      (Variables|Default|SetInferredVelocity (/ (- (Variables|Default|GetPrevRelativeLocation) (CallFunction|GetRelativeLocation)) (Utilities|Time|GetWorldDeltaSeconds)))
      (Variables|Default|SetPrevRelativeLocation (CallFunction|GetRelativeLocation)))
    (:then_2
      ;[1 1 1] Update shield collision
      (Collision|SetCollisionEnabled (Variables|Default|GetAttackSphere) (select (CallFunction|IsAttackActive) "QueryOnly" "NoCollision"))
      (Collision|SetCollisionEnabled (Variables|Default|GetDeflectionSphere) (select (not (CallFunction|IsAttackActive)) "QueryOnly" "NoCollision")))
    (:then_3
      ;[1 1 1] Update shield particle variables
      (Effects|Components|ParticleSystem|SetVectorParameter _shieldparticles "SpawnLocation" (CallFunction|GetRelativeLocation))
      (Effects|Components|ParticleSystem|SetFloatParameter _shieldparticles "Opacity" (Math|Float|MapRangeClamped (Math|Vector|VectorLength (Variables|Default|GetInferredVelocity)) (Variables|Default|GetAttackFadeInVelocityThreshold) (Variables|Default|GetAttackVelocityThreshold) 0.0 1.0))
      (Rendering|Material|SetScalarParameterValue (Variables|Default|GetRadialGradientMID) "Opacity" (- 1.0 (Math|Float|MapRangeClamped (Math|Vector|VectorLength (Variables|Default|GetInferredVelocity)) (Variables|Default|GetAttackFadeInVelocityThreshold) (Variables|Default|GetAttackVelocityThreshold) 0.0 1.0)) :!class /Script/Engine.MaterialInstanceDynamic))))

(event Collision|EventActorBeginOverlap
  (params (OtherActor :type Actor%20Object%20Reference))
  (bind _asbp_enemy (Utilities|Casting|CastToBP_Enemy OtherActor))
  (if (CallFunction|IsAttackActive)
    (Game|Damage|ApplyDamage _asbp_enemy 1.0 (Game|GetInstigatorController) self)))

(fn ConstructionScript)

(fn OnRepActiveHandComponent
  (Utilities|IsValid (Variables|Default|GetActiveHandComponent)
    (:Is%20Valid
      (Audio|Components|Audio|Stop (Variables|Default|GetAppearTimeline))
      (CallFunction|Disappear))))

(fn GetRelativeLocation
  (return (- (Transformation|GetActorLocation) (Transformation|GetActorLocation (Actor|GetAttachParentActor)))))

(fn IsAttackActive
  (return (>= (Math|Vector|VectorLength (Variables|Default|GetInferredVelocity)) (Variables|Default|GetAttackVelocityThreshold))))
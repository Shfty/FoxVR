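; BP_SpeedTransitionEvent is a spline event that, once triggered, eases the Fox VR pawn's spline velocity multiplier toward a target speed multiplier.
; Trigger sets a flag that lets Tick apply FInterpTo to the pawn's multiplier each frame.
; When the interpolated value is within tolerance of zero, rather than of the target, it snaps the multiplier to the target and destroys itself.
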(event EventTick
  (params (DeltaSeconds :type Float%20%28single-precision%29))
  (if (Variables|Default|GetTriggered)
    (bind _foxvr_pawn (Utilities|GetFoxVRPawn)
      (:Success
        (if (Math|Float|NearlyEqual(Float) (Math|Interpolation|FInterpTo (Variables|/Game/Blueprints/BP_FoxVRPawn.BP_FoxVRPawn_C|GetSplineVelocityMultiplier _foxvr_pawn) (Variables|Default|GetTargetSpeedMultiplier) (Utilities|Time|GetWorldDeltaSeconds) (Variables|Default|GetInterpSpeed)) 0.0 (Variables|Default|GetInterpCompleteTolerance))
          (Variables|/Game/Blueprints/BP_FoxVRPawn.BP_FoxVRPawn_C|SetSplineVelocityMultiplier _foxvr_pawn (Variables|Default|GetTargetSpeedMultiplier))
          (Actor|DestroyActor)
          (else
            (Variables|/Game/Blueprints/BP_FoxVRPawn.BP_FoxVRPawn_C|SetSplineVelocityMultiplier _foxvr_pawn (Math|Interpolation|FInterpTo (Variables|/Game/Blueprints/BP_FoxVRPawn.BP_FoxVRPawn_C|GetSplineVelocityMultiplier _foxvr_pawn) (Variables|Default|GetTargetSpeedMultiplier) (Utilities|Time|GetWorldDeltaSeconds) (Variables|Default|GetInterpSpeed)))))))))

(event EventTrigger
  (Variables|Default|SetTriggered true))

(fn ConstructionScript
  (|CallParentFunction))
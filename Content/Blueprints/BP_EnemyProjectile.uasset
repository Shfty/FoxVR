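; Enemy projectile that damages the player's plane or gets deflected by its defenses.
; On spawn it attaches to the player pawn, keeping its world transform.
; Overlapping a vulnerable BP_Plane deals damage and destroys the projectile, while an invincible plane or a BP_ArmorPod deflects it.
; Deflection sends it away from the source at fixed speed and sets a flag that disables further hits.
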(event Custom|Deflect
  (params (DeflectionSource :type Vector))
  (if (not (Variables|Default|GetDeflected))
    (Variables|/Script/Engine.MovementComponent|SetVelocity (Variables|Default|GetProjectileMovement) (* (Math|Vector|Normalize (- (Transformation|GetActorLocation) DeflectionSource)) 1e+03))
    (Variables|Default|SetDeflected true)))

(event EventBeginPlay
  (bind _returnvalue (Game|Player|GetPlayerPawn 0))
  (Utilities|IsValid _returnvalue
    (:Is%20Valid
      (Transformation|AttachActorToActor _returnvalue "None" "KeepWorld" "KeepWorld" "KeepWorld" false))))

(event Collision|EventActorBeginOverlap
  (params (OtherActor :type Actor%20Object%20Reference))
  (if (not (Variables|Default|GetDeflected))
    (bind _asbp_plane (Utilities|Casting|CastToBP_Plane OtherActor)
      (:then
        (if (Default|IsInvincible _asbp_plane)
          (CallFunction|Deflect (Transformation|GetActorLocation _asbp_plane))
          (else
            (Default|TakeDamage _asbp_plane 1)
            (Actor|DestroyActor))))
      (:CastFailed
        (bind _asbp_armor_pod (Utilities|Casting|CastToBP_ArmorPod OtherActor))
        (CallFunction|Deflect (Transformation|GetActorLocation _asbp_armor_pod))))))

(fn ConstructionScript)
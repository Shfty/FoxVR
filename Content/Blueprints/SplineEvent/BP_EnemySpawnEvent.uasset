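; BP_EnemySpawnEvent is an event actor that spawns enemies of a configured class when triggered.
; Trigger composes each SpawnTransforms entry with the actor's transform, spawns an EnemyClass instance there regardless of collision, and calls DestroyActor on itself inside the same loop.
; The construction script adds a billboard at each relative transform to mark the spawn points.
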(event EventTrigger
  (for _array_element (Variables|Default|GetSpawnTransforms)
    (Game|SpawnActorfromClass (Variables|Default|GetEnemyClass) (Math|Transform|ComposeTransforms _array_element (Transformation|GetActorTransform)) "AlwaysSpawn" 0 0)
    (Actor|DestroyActor)))

(fn ConstructionScript
  (|CallParentFunction)
  (for _array_element (Variables|Default|GetSpawnTransforms)
    (bind _returnvalue (AddComponent|AddBillboardComponent false _array_element))
    (Rendering|Components|Sprite|SetSprite _returnvalue "/Engine/EditorResources/S_Actor.S_Actor")))